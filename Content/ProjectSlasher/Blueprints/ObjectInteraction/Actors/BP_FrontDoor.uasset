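; Interactable front door that offers menu actions (walk, open, knock, cancel) to the top-down player through an action map and button names.
; Open or Knock runs at once if the player is inside the door's collision; otherwise it queues the action on the player controller and walks them over.
; On overlap, a queued action targeting this door is matched from string back to enum and executed.
; Open and Knock currently only print text and change the HUD menu.
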(event OnComponentBeginOverlap(DoorColision)
  (params (OverlappedComponent :type Primitive%20Component%20Object%20Reference) (OtherActor :type Actor%20Object%20Reference) (OtherComp :type Primitive%20Component%20Object%20Reference) (OtherBodyIndex :type Integer) (bFromSweep :type Boolean) (SweepResult :type Hit%20Result%20Structure%20%28by%20ref%29))
  (CallFunction|HandleComponentOverlap))

(event EventBeginPlay
  (bind _asbp_top_down_controller (Utilities|Casting|CastToBP_TopDownController (Game|GetPlayerController 0)))
  (Variables|Default|SetPlayerCtrlRef _asbp_top_down_controller))

(event EventObjAction
  (params (btnIndex :type Integer))
  (bind _self self)
  (bind _actionmap (Variables|Default|GetActionMap _self))
  (bind (_value _returnvalue) (Utilities|Map|Find _actionmap btnIndex))
  (if _returnvalue
    (CallFunction|HandleActionSelected _value)))

(fn ConstructionScript)

(fn HandleComponentOverlap
  (bind _playerisoverlapping (CallFunction|IsPlayerinCollision self (Variables|Default|GetDoorColision)))
  (if _playerisoverlapping
    (LocalVariables|SetQueuedAction (Variables|/Game/TopDown/Blueprints/BP_TopDownController.BP_TopDownController_C|GetCurrentQueuedAction (Variables|Default|GetPlayerCtrlRef)))
    (if (== self (.targetactor (LocalVariables|GetQueuedAction)))
      (Default|OnActionExecuted (Variables|Default|GetPlayerCtrlRef))
      (bind _chosenenum (CallFunction|GetChosenEnum (.objectaction (LocalVariables|GetQueuedAction))))
      (switch Utilities|FlowControl|Switch|SwitchonE_ObjectActions _chosenenum
        (:NewEnumerator1
          (CallFunction|HandleOpenAction))
        (:NewEnumerator0
          (CallFunction|HandleKnockAction))
        (:NewEnumerator4
          (return)))
      (return))))

(fn HandleActionSelected
  (params (SelectedAction :type E_ObjectActions%20Enum :default "NewEnumerator2"))
  (switch Utilities|FlowControl|Switch|SwitchonE_ObjectActions SelectedAction
    (:NewEnumerator2
      (Default|WalktoActorAction (Variables|Default|GetPlayerCtrlRef) true))
    (:NewEnumerator1
      (CallFunction|HandleOpenSelected))
    (:NewEnumerator0
      (CallFunction|HandleKnockSelected))
    (:NewEnumerator3
      (Default|ChangeMenu (Variables|/Game/TopDown/Blueprints/BP_TopDownController.BP_TopDownController_C|GetHudRef (Variables|Default|GetPlayerCtrlRef)) true))))

(fn HandleOpenSelected
  (bind _playerisoverlapping (CallFunction|IsPlayerinCollision self (Variables|Default|GetDoorColision)))
  (if _playerisoverlapping
    (CallFunction|HandleOpenAction)
    (else
      (Default|UpdateQueuedAction (Variables|Default|GetPlayerCtrlRef) (Utilities|Struct|MakeF_Player_Action (Utilities|String|EnumtoString (Utilities|Enum|LiteralenumE_ObjectActions "NewEnumerator1")) self))
      (Default|WalktoActorAction (Variables|Default|GetPlayerCtrlRef) true))))

(fn HandleKnockSelected
  (bind _playerisoverlapping (CallFunction|IsPlayerinCollision self (Variables|Default|GetDoorColision)))
  (if _playerisoverlapping
    (CallFunction|HandleKnockAction)
    (else
      (Default|UpdateQueuedAction (Variables|Default|GetPlayerCtrlRef) (Utilities|Struct|MakeF_Player_Action (Utilities|String|EnumtoString (Utilities|Enum|LiteralenumE_ObjectActions "NewEnumerator0")) self))
      (Default|WalktoActorAction (Variables|Default|GetPlayerCtrlRef) true))))

(fn HandleOpenAction
  (Development|PrintString "Opening")
  (Default|ChangeMenu (Variables|/Game/TopDown/Blueprints/BP_TopDownController.BP_TopDownController_C|GetHudRef (Variables|Default|GetPlayerCtrlRef)) true))

(fn HandleKnockAction
  (Development|PrintString "Knock Knock Knocking on Slahers Door")
  (Default|ChangeMenu (Variables|/Game/TopDown/Blueprints/BP_TopDownController.BP_TopDownController_C|GetHudRef (Variables|Default|GetPlayerCtrlRef)) true))

(fn GetChosenEnum
  (params (ChosenAction :type String))
  (bind _values (Utilities|Map|Values (Variables|Default|GetActionMap)))
  (bind _array_element (Utilities|Array|ForEachLoopwithBreak _values)
    (:LoopBody
      (if (Utilities|Enum|Equal(Enum) (Utilities|String|EnumtoString _array_element) ChosenAction)
        (return _array_element)))
    (:Completed
      (return "NewEnumerator4"))))

(fn GetButtonActions
  (return (Variables|Default|GetActionMap)))

(fn GetButtonNames
  (return (Variables|Default|GetBtnNamesArray)))