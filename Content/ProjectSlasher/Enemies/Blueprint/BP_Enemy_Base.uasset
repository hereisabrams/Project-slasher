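; Base enemy character Blueprint with a scare meter and animated activities such as picking up, sleeping, watching TV and investigating.
; Tick pushes the scare value and state image into the overhead or attached ScareBar widget.
; Each activity event plays a montage, then fires its end dispatcher on either completion or interruption.
; Helper functions expose the patrol route and map speed states to max walk speed.
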(event Custom|Pick
  (Animation|Montage|PlayMontage (Variables|Character|GetMesh) "/Game/ProjectSlasher/Enemies/Animations/PickUp_UE_Montage.PickUp_UE_Montage"
    (:OnCompleted
      _)
    (:OnInterrupted
      _))
  (Default|CallOnPickEnd))

(event Custom|Get%20To%20Bed
  (Animation|Montage|PlayMontage (Variables|Character|GetMesh) "/Game/ProjectSlasher/Enemies/Animations/LyingDown_UE_Montage.LyingDown_UE_Montage"
    (:OnCompleted
      _)
    (:OnInterrupted
      _))
  (Default|CallOnGettoBedEnd))

(event Custom|Wake%20From%20Bed
  (Animation|Montage|PlayMontage (Variables|Character|GetMesh) "/Game/ProjectSlasher/Enemies/Animations/GettingUp_UE_Montage.GettingUp_UE_Montage"
    (:OnCompleted
      _)
    (:OnInterrupted
      _))
  (Default|CallOnWakefromBedEnd))

(event Custom|Watch%20TV
  (Animation|Montage|PlayMontage (Variables|Character|GetMesh) "/Game/ProjectSlasher/Enemies/Animations/OverheadSquat_UE_Montage.OverheadSquat_UE_Montage"
    (:OnCompleted
      _)
    (:OnInterrupted
      _))
  (Default|CallOnWatchTVEnd))

(event Custom|Start%20Investigating
  (Animation|Montage|PlayMontage (Variables|Character|GetMesh) "/Game/ProjectSlasher/Enemies/Animations/PickUp_UE_Montage.PickUp_UE_Montage"
    (:OnCompleted
      _)
    (:OnInterrupted
      _))
  (Default|CallOnStartInvestingatingEnd))

(event EventTick
  (params (DeltaSeconds :type Float%20%28single-precision%29))
  (bind _aswb_scared_bar (Utilities|Casting|CastToWB_ScaredBar (UserInterface|GetWidget (Variables|Default|GetScare%20Bar%20Widget))))
  (Variables|/Script/UMG.ProgressBar|SetPercent (Variables|/Game/ProjectSlasher/Enemies/Interface/WB_ScaredBar.WB_ScaredBar_C|GetScareBar _aswb_scared_bar) (Variables|Default|GetScaredMeter))
  (Class|Image|SetBrush (Variables|/Game/ProjectSlasher/Enemies/Interface/WB_ScaredBar.WB_ScaredBar_C|GetImageState _aswb_scared_bar) (Variables|Default|GetIn%20Brush)))

(fn ConstructionScript)

(fn GetPatrolRoute
  (return (Variables|AI|GetPatrolRoute)))

(fn SetMovementSpeed
  (params (Speed :type E_Speed%20Enum :default "NewEnumerator0"))
  (bind _output_get (Variables|/Script/Engine.CharacterMovementComponent|SetMaxWalkSpeed (Variables|Character|GetCharacterMovement) (Utilities|Select :Index Speed :NewEnumerator0 0.0 :NewEnumerator1 1e+02 :NewEnumerator2 3e+02 :NewEnumerator3 6e+02)))
  (return _output_get))